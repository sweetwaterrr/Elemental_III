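; Meteor ability actor that flies from its spawn point to the player's cursor location and spawns impact effects there.
; On BeginPlay it caches both positions, then a timeline drives a non-sweeping location lerp between them.
; The timeline's Hit event, rather than collision, triggers SpawnGE for the meteor hit and debris classes at the target.
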(event EventBeginPlay
  (|CallParentFunction)
  (Variables|Default|SetInitialPos (Transformation|GetActorLocation))
  (Variables|Default|SetTargetPos (.location (Variables|/Game/TAcourse_III/GameBP/Pawn/Player/B_ElementalPlayer.B_ElementalPlayer_C|GetCursorData (Variables|Default|GetElementalPlayer))))
  (bind _motion (Timeline|Animation Play)
    (:Update
      (Transformation|SetActorLocation (Math|Vector|Lerp(Vector) (Variables|Default|GetInitialPos) (Variables|Default|GetTargetPos) _motion) false false))
    (:Hit
      (CallFunction|SpawnGE "/Game/TAcourse_III/Ability/Fire_Meteor/GA_MeteorHit.GA_MeteorHit_C" (Math|Transform|MakeTransform (Variables|Default|GetTargetPos)) false true 0 5.0)
      (CallFunction|SpawnGE "/Game/TAcourse_III/Ability/Fire_Meteor/GA_Debris.GA_Debris_C" (Math|Transform|MakeTransform (Variables|Default|GetTargetPos)) false true 0 5.0))))

(event Collision|EventActorBeginOverlap
  (params (OtherActor :type Actor%20Object%20Reference))
  (|CallParentFunction OtherActor) ; This node is disabled and will not be called.\nDrag off pins to build functionality.
)

(event EventTick
  (params (DeltaSeconds :type Float%20%28single-precision%29))
  (|CallParentFunction DeltaSeconds) ; This node is disabled and will not be called.\nDrag off pins to build functionality.
)

(fn ConstructionScript
  (|CallParentFunction))