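; Fire meteor ability that spawns a GA_Meteor above the player's cursor location when the ability key is released.
; On release, CFCdCheck gates the cast, then CFApplyCd starts the cooldown and SpawnGE creates the meteor.
; The spawn point is offset from the cursor along a random direction in an upward cone, scaled by DistancetoTarget, so each meteor's origin varies.
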(event EventBeginPlay
  (|CallParentFunction) ; This node is disabled and will not be called.\nDrag off pins to build functionality.
)

(event Collision|EventActorBeginOverlap
  (params (OtherActor :type Actor%20Object%20Reference)))

(event EventTick
  (params (DeltaSeconds :type Float%20%28single-precision%29)))

(event EventCEKeyReleased
  ;[1 1 1] 默认情况下, 松开按键视为 cast 技能 并检查和设置CD
  (bind _cd (CallFunction|CFCdCheck))
  (if (not _cd)
    (CallFunction|CFApplyCd)
    (CallFunction|SpawnGE "/Game/TAcourse_III/Ability/Fire_Meteor/GA_Meteor.GA_Meteor_C" (Math|Transform|MakeTransform (+ (.location (Variables|/Game/TAcourse_III/GameBP/Pawn/Player/B_ElementalPlayer.B_ElementalPlayer_C|GetCursorData (Variables|Default|GetElementalPlayer))) (* (Math|Random|RandomUnitVectorinConeinDegrees "0, 0,1.000000" (Variables|Default|GetCone%20Half%20Angle%20in%20Degrees)) (Variables|Default|GetDistancetoTarget)) "")) true true 0 5.0)))

(fn ConstructionScript
  (|CallParentFunction))